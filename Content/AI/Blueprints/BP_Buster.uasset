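; BP_Buster is a damageable AI actor that replaces itself with a fresh copy when killed.
; It starts at MaxHealth, and any damage sets PlayerFound and reduces health while alive.
; At zero health it sets IsDead and calls Respawn, which spawns a new BP_Buster at a random ground-plane position with fixed height, destroys itself and prints a kill message.
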(event EventBeginPlay
  (Variables|Default|SetCurrentHealth (Variables|Default|GetMaxHealth)))

(event EventTakeDamage
  (params (BoneName :type Name :default "None") (Damage :type Float%20%28single-precision%29))
  (Variables|Default|SetPlayerFound true)
  (if (not (Variables|Default|GetisDead))
    (bind _output_get (Variables|Default|SetCurrentHealth (- (Variables|Default|GetCurrentHealth) Damage)))
    (if (<= _output_get 0.0)
      (Variables|Default|SetisDead (<= _output_get 0.0))
      (CallFunction|Respawn))))

(fn ConstructionScript)

(fn Respawn
  (Game|SpawnActorfromClass "BP_Buster_C" (Math|Transform|MakeTransform (Math|Vector|MakeVector (Math|Random|RandomFloatinRange -5e+03 0.0) (Math|Random|RandomFloatinRange 5e+03 0.0) 1.2e+02)) "AlwaysSpawn" 0 0)
  (Actor|DestroyActor)
  (Development|PrintString "Kill"))