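; AR4 rifle weapon Blueprint with a 24-round magazine, fired by the player's BP_Manny character.
; Fire decrements ammo, switching the player from firing to reloading at zero, then always runs the shot without gating on ammo.
; A debug-drawn camera trace stores hit data and aims a BP_AR4Projectile spawned at the muzzle socket toward the impact point, or the trace end on a miss.
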(event EventFire
  (CallFunction|AmmoCounter)
  (CallFunction|ShootLineTrace))

(fn ConstructionScript
  (|CallParentFunction)
  (Variables|Default|SetAmmoCount 24)
  (Variables|Default|SetMaxAmmo 24))

(fn AmmoCounter
  (bind _returnvalue (Game|GetPlayerCharacter 0))
  (bind _asbp_manny (Utilities|Casting|CastToBP_Manny _returnvalue))
  (if (> (Variables|Default|GetAmmoCount) 0)
    (bind _result (Math|Integer|DecrementInt (Variables|Default|GetAmmoCount))
      (:%20%20
        (if (<= _result 0)
          (Variables|/Game/Character/Blueprints/Manny/BP_Manny.BP_Manny_C|SetisFiring _asbp_manny false)
          (Variables|/Game/Character/Blueprints/Manny/BP_Manny.BP_Manny_C|SetisReloading _asbp_manny true))))))

(fn ShootLineTrace
  (bind _returnvalue (Game|GetPlayerCharacter 0))
  (bind _skeletalmesh (Variables|Default|GetSkeletalMesh))
  (bind _returnvalue_2 (Transformation|GetSocketLocation _skeletalmesh "MuzzleFlashSocket"))
  (bind _asbp_manny (Utilities|Casting|CastToBP_Manny _returnvalue))
  (bind _camera (Variables|/Game/Character/Blueprints/Manny/BP_Manny.BP_Manny_C|GetCamera _asbp_manny))
  (bind _returnvalue_3 (Transformation|GetWorldLocation _camera))
  (bind (_outhit _returnvalue_4) (Collision|LineTraceByChannel _returnvalue_3 (+ _returnvalue_3 (* (Math|Vector|GetForwardVector _camera) 2.5e+04)) "TraceTypeQuery1" false 0 "ForDuration"))
  (Variables|Default|SetLocation (.Location (Collision|BreakHitResult _outhit)))
  (Variables|Default|SetImpactPoint (.ImpactPoint (Collision|BreakHitResult _outhit)))
  (bind _output_get (Variables|Default|SetImpactNormal (.ImpactNormal (Collision|BreakHitResult _outhit))))
  (bind _output_get_2 (Variables|Default|SetHitActor (.HitActor (Collision|BreakHitResult _outhit))))
  (Variables|Default|SetHitComponent (.HitComponent (Collision|BreakHitResult _outhit)))
  (Variables|Default|SetHitBoneName (.HitBoneName (Collision|BreakHitResult _outhit)))
  (Variables|Default|SetTraceStart (.TraceStart (Collision|BreakHitResult _outhit)))
  (bind _output_get_3 (Variables|Default|SetTraceEnd (.TraceEnd (Collision|BreakHitResult _outhit))))
  (Variables|Default|SetHitNormalRotation (Math|Conversions|RotationFromXVector _output_get))
  (Variables|Default|SetHitActorClass (Utilities|GetClass _output_get_2))
  (Game|SpawnActorfromClass "/Game/Weapons/BP_AR4Projectile.BP_AR4Projectile_C" (Math|Transform|MakeTransform _returnvalue_2 (Math|Rotator|FindLookatRotation _returnvalue_2 (Math|Vector|SelectVector (Variables|Default|GetImpactPoint) _output_get_3 _returnvalue_4))) "AlwaysSpawn" 0 0))